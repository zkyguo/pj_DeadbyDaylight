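; Player start for a Dead by Daylight-style mode, flagged by IsDemon as either a demon or non-demon spawn.
; The construction script tints the cone red for demon starts and green otherwise, and makes the cube transparent for demons or semi-opaque for others.
; It also scales the cube horizontally by CharacterStartSize.
; The event graph holds no active logic.
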(fn `UserConstructionScript`
  (bind _cube (`self.Cube`))
  (bind _returnvalue (`KismetMathLibrary.Conv_IntToDouble` (`self.CharacterStartSize`)))
  (`MeshComponent.SetVectorParameterValueOnMaterials` (`self.Cone`) "Color" (select `bool` (`self.bIsDemon`) :`false` (0.0 1.0 0.0) :`true` (1.0 0.0 0.0) :!type "Vector Structure"))
  (`MeshComponent.SetScalarParameterValueOnMaterials` _cube "Opacity" (select `bool` (`self.bIsDemon`) :`false` 0.5 :!type "Float (single-precision)"))
  (`SceneComponent.SetRelativeScale3D` _cube (`KismetMathLibrary.MakeVector` _returnvalue _returnvalue 1.0)))